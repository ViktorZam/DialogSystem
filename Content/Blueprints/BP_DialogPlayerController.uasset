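; Player controller that drives dialog input between the player and the BP_AI character through the HUD's main interface widget.
; Holding F while the dialog indicator shows opens the answer list, and the mouse wheel cycles the selection.
; Releasing F matches the hard-coded Russian yes/no text to DT_Answers rows by index and continues the AI's dialog, or restores the indicator on ellipsis if overlapping.
; E advances dialog in one specific AI status.
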(event `Key|G`
  (params (Key :type "Key Structure")))

(event `self.ReceiveBeginPlay`
  (bind _asbp_hud (cast `/Game/Blueprints/BP_HUD` (`self.GetHUD`)))
  (set `self.HUD` _asbp_hud))

(event `Key|F`
  (params (Key :type "Key Structure"))
  (:`Pressed`
    (if (`|EnumEquality` (`Widget.GetVisibility` (`/Game/Widgets/WBP_MainInterface.Image_DialogIndicator` (`/Game/Blueprints/BP_HUD.MainInterfaceWidget` (`self.HUD`)))) "Visible")
      (`Widget.SetVisibility` (`/Game/Widgets/WBP_MainInterface.Image_DialogIndicator` (`/Game/Blueprints/BP_HUD.MainInterfaceWidget` (`self.HUD`))) "Collapsed")
      (`Widget.SetVisibility` (`/Game/Widgets/WBP_MainInterface.VerticalBox_Answers` (`/Game/Blueprints/BP_HUD.MainInterfaceWidget` (`self.HUD`))) "SelfHitTestInvisible")))
  (:`Released`
    (if (`|EnumEquality` (`Widget.GetVisibility` (`/Game/Widgets/WBP_MainInterface.VerticalBox_Answers` (`/Game/Blueprints/BP_HUD.MainInterfaceWidget` (`self.HUD`)))) "SelfHitTestInvisible")
      (`Widget.SetVisibility` (`/Game/Widgets/WBP_MainInterface.VerticalBox_Answers` (`/Game/Blueprints/BP_HUD.MainInterfaceWidget` (`self.HUD`))) "Collapsed")
      (switch `string` (`/Game/Widgets/WBP_MainInterface.Answer` (`/Game/Blueprints/BP_HUD.MainInterfaceWidget` (`self.HUD`)))
        (:`ДА, ПОЙДЁМ`
          (bind _returnvalue (`GameplayStatics.GetActorOfClass` "/Game/Blueprints/BP_AI.BP_AI_C"))
          (bind _outrownames (`DataTableFunctionLibrary.GetDataTableRowNames` "/Game/Data/DT_Answers.DT_Answers"))
          (bind _returnvalue_2 (`|GetDataTableRow` "/Game/Data/DT_Answers.DT_Answers" (`|GetArrayItem` _outrownames))
            (:`then`
              (set `/Game/Blueprints/BP_AI.CurrentDialog` (`.DialogAI_8_0B6DC32947CE6EFBC1ADAD842E6AB4A0` (break `/Game/Data/S_Dialog` _returnvalue_2)) _returnvalue)
              (set `/Game/Blueprints/BP_AI.CurrentStatusAI` "NewEnumerator4" _returnvalue)
              (`/Game/Blueprints/BP_AI.ContinueDialog` _returnvalue false))))
        (:`НЕТ, ТУДА НЕЛЬЗЯ`
          (bind _returnvalue_3 (`GameplayStatics.GetActorOfClass` "/Game/Blueprints/BP_AI.BP_AI_C"))
          (bind _outrownames_2 (`DataTableFunctionLibrary.GetDataTableRowNames` "/Game/Data/DT_Answers.DT_Answers"))
          (bind _returnvalue_4 (`|GetDataTableRow` "/Game/Data/DT_Answers.DT_Answers" (`|GetArrayItem` _outrownames_2 1))
            (:`then`
              (set `/Game/Blueprints/BP_AI.CurrentDialog` (`.DialogAI_8_0B6DC32947CE6EFBC1ADAD842E6AB4A0` (break `/Game/Data/S_Dialog` _returnvalue_4)) _returnvalue_3)
              (set `/Game/Blueprints/BP_AI.CurrentStatusAI` "NewEnumerator4" _returnvalue_3)
              (`/Game/Blueprints/BP_AI.ContinueDialog` _returnvalue_3 false))))
        (:`. . .`
          (if (!= (`KismetArrayLibrary.Array_Length` (`self.GetOverlappingActors` (`self.K2_GetPawn`) "/Game/Blueprints/BP_AI.BP_AI_C")) 0)
            (`Widget.SetVisibility` (`/Game/Widgets/WBP_MainInterface.Image_DialogIndicator` (`/Game/Blueprints/BP_HUD.MainInterfaceWidget` (`self.HUD`))) "Visible")))))))

(event `Key|E`
  (params (Key :type "Key Structure"))
  (:`Pressed`
    (bind _returnvalue (`GameplayStatics.GetActorOfClass` "/Game/Blueprints/BP_AI.BP_AI_C"))
    (if (`|EnumEquality` (`/Game/Blueprints/BP_AI.CurrentStatusAI` _returnvalue) "NewEnumerator3")
      (set `/Game/Blueprints/BP_AI.CurrentStatusAI` "NewEnumerator4" _returnvalue)
      (`/Game/Blueprints/BP_AI.ContinueDialog` _returnvalue false))))

(event `Key|MouseScrollUp`
  (params (Key :type "Key Structure"))
  (:`Pressed`
    (if (`|EnumEquality` (`Widget.GetVisibility` (`/Game/Widgets/WBP_MainInterface.VerticalBox_Answers` (`/Game/Blueprints/BP_HUD.MainInterfaceWidget` (`self.HUD`)))) "SelfHitTestInvisible")
      (`/Game/Widgets/WBP_MainInterface.ChoisingAnswer` (`/Game/Blueprints/BP_HUD.MainInterfaceWidget` (`self.HUD`)) true))))

(event `Key|MouseScrollDown`
  (params (Key :type "Key Structure"))
  (:`Pressed`
    (if (`|EnumEquality` (`Widget.GetVisibility` (`/Game/Widgets/WBP_MainInterface.VerticalBox_Answers` (`/Game/Blueprints/BP_HUD.MainInterfaceWidget` (`self.HUD`)))) "SelfHitTestInvisible")
      (`/Game/Widgets/WBP_MainInterface.ChoisingAnswer` (`/Game/Blueprints/BP_HUD.MainInterfaceWidget` (`self.HUD`)) false))))

(fn `UserConstructionScript`)