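; NPC that talks to the player through a world-space dialogue widget and walks a BP_Splain spline.
; Overlapping its box starts DataTable dialogue or offers answers through the player controller, with a status enum sequencing lines, waits and movement.
; Timers and falling hits trigger interrupting reaction lines when the player lingers, strays or jumps on it.
; A speed-scaled timeline feeds AI MoveTo along the spline, pausing when PawnSensing sees a pawn.
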(event `ContinueMoving`
  (`Timeline|Timeline_SplineMoving` :!label _label
    (:`Update`
      (`|AIMoveTo` self (`SplineComponent.GetLocationAtTime` (`self.SplinePath`) (`KismetMathLibrary.NormalizeToRange` (`TimelineComponent.GetPlaybackPosition` (`self.Timeline_SplineMoving`)) 0.0 (* (/ (`SplineComponent.GetSplineLength` (`self.SplinePath`)) (`CharacterMovementComponent.MaxWalkSpeed` (`self.CharacterMovement`))) 1.3)) "World" true) null 1.0))))

(event `self.ReceiveBeginPlay`
  (bind _returnvalue (`GameplayStatics.GetActorOfClass` "/Game/Blueprints/BP_Splain.BP_Splain_C"))
  (set `self.SplinePath` (`/Game/Blueprints/BP_Splain.Spline` _returnvalue))
  (bind _movementresult (`|AIMoveTo` self (0.0 0.0 0.0) _returnvalue 1.0)
    (:`OnSuccess`
      _)
    (:`OnFail`
      (switch `EPathFollowingResult` _movementresult
        (:`Aborted`
          _))))
  (`TimelineComponent.SetTimelineLength` (`self.Timeline_SplineMoving`) (* (/ (`SplineComponent.GetSplineLength` (`self.SplinePath`)) (`CharacterMovementComponent.MaxWalkSpeed` (`self.CharacterMovement`))) 1.3)))

(event `StopMoving`
  (`NavMovementComponent.StopActiveMovement` (`self.CharacterMovement`))
  (goto _label :!via `Stop`))

(event `self.ReceiveTick`
  (params (DeltaSeconds :type "Float (single-precision)"))
  (if (not (`SceneComponent.bHiddenInGame` (`self.Widget`)))
    (bind _returnvalue (`GameplayStatics.GetActorOfClass` "/Game/Blueprints/BP_CapsuleCharacter.BP_CapsuleCharacter_C"))
    (bind (_returnvalue_roll _returnvalue_pitch _returnvalue_yaw) (`KismetMathLibrary.BreakRotator` (`self.GetControlRotation` _returnvalue)))
    (`SceneComponent.K2_SetWorldRotation` (`self.Widget`) (`KismetMathLibrary.MakeRotator` 0.0 0.0 (+ (`KismetMathLibrary.NormalizeAxis` _returnvalue_yaw) 180.0)) false false)))

(event `StartBeginDialog`
  (switch `/Game/Data/E_StatusAI` (`self.CurrentStatusAI`) :!label _label_2
    (:`NewEnumerator1`
      (`/Engine/EditorBlueprintResources/StandardMacros.DoOnce` false :!label _label_3
        (:`Completed`
          (`self.StartCheckPlayer`)
          (bind _aswbp_dialog_window (cast `/Game/Widgets/WBP_DialogWindow` (`WidgetComponent.GetUserWidgetObject` (`self.Widget`))))
          (`Widget.SetVisibility` (`/Game/Widgets/WBP_DialogWindow.SizeBox_Message` _aswbp_dialog_window) "Hidden")
          (bind _returnvalue (`|GetDataTableRow` (`self.CurrentDialog`) "1")
            (:`then`
              (bind _message (break `/Game/Data/S_Dialog` _returnvalue))
              (`TextBlock.SetText` (`/Game/Widgets/WBP_DialogWindow.TextBlock_TestMessage` _aswbp_dialog_window) (`KismetTextLibrary.Conv_StringToText` _message))
              (`Border.SetBrushColor` :`self` (`/Game/Widgets/WBP_DialogWindow.Border_BackGround` _aswbp_dialog_window))
              (`KismetSystemLibrary.Delay` 0.2)
              (`/Game/Widgets/WBP_DialogWindow.SayMessage` _aswbp_dialog_window _message self "NewEnumerator0" false))))))
    (:`NewEnumerator0`
      (bind _asbp_dialog_player_controller (cast `/Game/Blueprints/BP_DialogPlayerController` (`GameplayStatics.GetPlayerController` 0)))
      (set `/Game/Blueprints/BP_DialogPlayerController.Answers` (`self.Answers`) _asbp_dialog_player_controller)
      (`Widget.SetVisibility` (`/Game/Widgets/WBP_MainInterface.Image_DialogIndicator` (`/Game/Blueprints/BP_HUD.MainInterfaceWidget` (`/Game/Blueprints/BP_DialogPlayerController.HUD` _asbp_dialog_player_controller))) "Visible"))))

(event `self.Box.OnComponentBeginOverlap`
  (params (OverlappedComponent :type "PrimitiveComponent Object Reference") (OtherActor :type "Actor Object Reference") (OtherComp :type "PrimitiveComponent Object Reference") (OtherBodyIndex :type Integer) (bFromSweep :type Boolean) (SweepResult :type "HitResult Structure (by ref)"))
  (if (!= OtherActor self)
    (goto _label_2)))

(event `ResetStartDialog`
  (goto _label_3 :!via `Reset`))

(event `self.Box.OnComponentEndOverlap`
  (params (OverlappedComponent :type "PrimitiveComponent Object Reference") (OtherActor :type "Actor Object Reference") (OtherComp :type "PrimitiveComponent Object Reference") (OtherBodyIndex :type Integer))
  (if (!= OtherActor self)
    (bind _asbp_dialog_player_controller (cast `/Game/Blueprints/BP_DialogPlayerController` (`GameplayStatics.GetPlayerController` 0)))
    (set `/Game/Blueprints/BP_DialogPlayerController.Answers` null _asbp_dialog_player_controller)
    (`Widget.SetVisibility` (`/Game/Widgets/WBP_MainInterface.Image_DialogIndicator` (`/Game/Blueprints/BP_HUD.MainInterfaceWidget` (`/Game/Blueprints/BP_DialogPlayerController.HUD` _asbp_dialog_player_controller))) "Collapsed")))

(event `ContinueDialog`
  (params (`SayReactionReplica?` :type Boolean))
  (`/Engine/EditorBlueprintResources/StandardMacros.IsValid` (`self.CurrentDialog`)
    (:`Is Valid`
      (`Border.SetBrushColor` (`/Game/Widgets/WBP_DialogWindow.Border_BackGround` (cast `/Game/Widgets/WBP_DialogWindow` (`WidgetComponent.GetUserWidgetObject` (`self.Widget`)) :!pure true)) (struct :`A` 1.0))
      (bind _result (`/Engine/EditorBlueprintResources/StandardMacros.IncrementInt` (`self.NumDialog`) :!label _label_4)
        (:`  `
          (bind _returnvalue (`|GetDataTableRow` (`self.CurrentDialog`) (`KismetStringLibrary.Conv_StringToName` (`KismetStringLibrary.Conv_IntToString` _result)))
            (:`then`
              (bind (_message _numnextmessage _dialogai _statusai) (break `/Game/Data/S_Dialog` _returnvalue))
              (if (!= _numnextmessage 0)
                (if (or (`|EnumInequality` _statusai "NewEnumerator5") `SayReactionReplica?`)
                  (bind _aswbp_dialog_window (cast `/Game/Widgets/WBP_DialogWindow` (`WidgetComponent.GetUserWidgetObject` (`self.Widget`))))
                  (`TextBlock.SetText` (`/Game/Widgets/WBP_DialogWindow.TextBlock_TestMessage` _aswbp_dialog_window) (`KismetTextLibrary.Conv_StringToText` _message))
                  (`KismetSystemLibrary.Delay` 0.2)
                  (if (`|EnumInequality` _statusai "NewEnumerator0")
                    (`/Game/Widgets/WBP_DialogWindow.SayMessage` (cast `/Game/Widgets/WBP_DialogWindow` (`WidgetComponent.GetUserWidgetObject` (`self.Widget`)) :!pure true) _message self "NewEnumerator3" false)
                    (else
                      (set `self.NumDialog` 0)
                      (`/Game/Widgets/WBP_DialogWindow.SayMessage` (cast `/Game/Widgets/WBP_DialogWindow` (`WidgetComponent.GetUserWidgetObject` (`self.Widget`)) :!pure true) _message self "NewEnumerator0" false)))
                  (else
                    (goto _label_4)))
                (else
                  (set `self.CurrentStatusAI` _statusai)
                  (set `self.NumDialog` 0 :!label _label_5)
                  (switch `/Game/Data/E_StatusAI` (`self.CurrentStatusAI`)
                    (:`NewEnumerator0`
                      (if (> (`KismetArrayLibrary.Array_Length` (`PrimitiveComponent.GetOverlappingActors` (`self.Box`) "/Game/Blueprints/BP_CapsuleCharacter.BP_CapsuleCharacter_C")) 0)
                        (bind _asbp_dialog_player_controller (cast `/Game/Blueprints/BP_DialogPlayerController` (`GameplayStatics.GetPlayerController` 0)))
                        (set `/Game/Blueprints/BP_DialogPlayerController.Answers` (`self.Answers`) _asbp_dialog_player_controller)
                        (`Widget.SetVisibility` (`/Game/Widgets/WBP_MainInterface.Image_DialogIndicator` (`/Game/Blueprints/BP_HUD.MainInterfaceWidget` (`/Game/Blueprints/BP_DialogPlayerController.HUD` _asbp_dialog_player_controller))) "Visible")))
                    (:`NewEnumerator2`
                      (bind _aswbp_dialog_window_2 (cast `/Game/Widgets/WBP_DialogWindow` (`WidgetComponent.GetUserWidgetObject` (`self.Widget`))))
                      (`KismetSystemLibrary.Delay` 1.0)
                      (`Widget.SetVisibility` (`/Game/Widgets/WBP_DialogWindow.SizeBox_Message` _aswbp_dialog_window_2) "Hidden")
                      (`self.ContinueMoving`))))))))))
    (:`Is Not Valid`
      (set `self.CurrentStatusAI` (`self.LastStatusAI`))
      (goto _label_5))))

(event `self.CapsuleComponent.OnComponentHit`
  (params (HitComponent :type "PrimitiveComponent Object Reference") (OtherActor :type "Actor Object Reference") (OtherComp :type "PrimitiveComponent Object Reference") (NormalImpulse :type "Vector Structure") (Hit :type "HitResult Structure (by ref)"))
  (bind _asbp_capsule_character (cast `/Game/Blueprints/BP_CapsuleCharacter` OtherActor))
  (if (`NavMovementComponent.IsFalling` (`Character.CharacterMovement` _asbp_capsule_character))
    (`/Engine/EditorBlueprintResources/StandardMacros.DoOnce` false :!label _label_6
      (:`Completed`
        (set `self.LastStatusAI` (`self.CurrentStatusAI`))
        (if (not (`|EnumInequality` (`self.LastStatusAI`) "NewEnumerator2"))
          (`self.StopMoving`)
          (set `self.CurrentDialog` null))
        (`self.HandlerReaction` "2" "NewEnumerator3")
        (`self.ResetJumpOnAI`)))))

(event `ResetJumpOnAI`
  (goto _label_6 :!via `Reset`))

(event `StartCheckPlayer`
  (bind _returnvalue (`GameplayStatics.GetActorOfClass` "/Game/Blueprints/BP_CapsuleCharacter.BP_CapsuleCharacter_C"))
  (set `self.LastSaveDistanceToPlayer` (`KismetMathLibrary.Vector_Distance` (`self.K2_GetActorLocation` _returnvalue) (`self.K2_GetActorLocation`)))
  (bind _returnvalue_2 (`KismetSystemLibrary.K2_SetTimerDelegate` (delegate `CheckPlayer`) 8.0))
  (set `self.TimerCheckPlayer` _returnvalue_2)
  (bind _returnvalue_3 (`KismetSystemLibrary.K2_SetTimerDelegate` (delegate `CheckDistance`) 1.0 true))
  (set `self.TimerCheckDistanceToPlayer` _returnvalue_3))

(event `CheckDistance`
  (bind _returnvalue (`GameplayStatics.GetActorOfClass` "/Game/Blueprints/BP_CapsuleCharacter.BP_CapsuleCharacter_C"))
  (if (> (`KismetMathLibrary.Vector_Distance` (`self.K2_GetActorLocation` _returnvalue) (`self.K2_GetActorLocation`)) 1000.0)
    (switch `/Game/Data/E_StatusAI` (`self.CurrentStatusAI`)
      (:`NewEnumerator1`
        _)
      (:`NewEnumerator0`
        _)
      (:`NewEnumerator2`
        (`self.StopMoving`)
        (set `self.CurrentDialog` null))
      (:`NewEnumerator3`
        _)
      (:`NewEnumerator4`
        _))
    (set `self.LastStatusAI` (`self.CurrentStatusAI`))
    (`self.ResetContinueDialog`)
    (`self.HandlerReaction` "4" "NewEnumerator5")
    (else
      (switch `/Game/Data/E_StatusAI` (`self.CurrentStatusAI`)
        (:`NewEnumerator5`
          (`/Engine/EditorBlueprintResources/StandardMacros.DoOnce` true :!label _label_7
            (:`Completed`
              (`self.ContinueDialog` false))))))))

(event `CheckPlayer`
  (bind _returnvalue (`GameplayStatics.GetActorOfClass` "/Game/Blueprints/BP_CapsuleCharacter.BP_CapsuleCharacter_C"))
  (if (and (== (`KismetMathLibrary.Vector_Distance` (`self.K2_GetActorLocation` _returnvalue) (`self.K2_GetActorLocation`)) (`self.LastSaveDistanceToPlayer`)) (`|EnumEquality` (`self.CurrentStatusAI`) "NewEnumerator0"))
    (`self.HandlerReaction` "1" "NewEnumerator3")
    (elif (`|EnumEquality` (`self.CurrentStatusAI`) "NewEnumerator0")
      (`self.HandlerReaction` "3" "NewEnumerator3"))))

(event `ResetContinueDialog`
  (goto _label_7 :!via `Reset`))

(event `self.PawnSensing.OnSeePawn`
  (params (Pawn :type "Pawn Object Reference"))
  (if (`|EnumEquality` (`self.CurrentStatusAI`) "NewEnumerator2")
    (`self.StopMoving`)
    (`KismetSystemLibrary.RetriggerableDelay` 2.0)
    (`self.ContinueMoving`)))

(fn `FindReactionReplicaInCurrentDialog`
  (returns (`Having?` :type Boolean))
  (locals (`LHaveReactionReplica?` :type Boolean))
  (bind _outrownames (`DataTableFunctionLibrary.GetDataTableRowNames` (`self.CurrentDialog`)))
  (for (_array_element _array_index) _outrownames
    (bind _returnvalue (`|GetDataTableRow` (`self.CurrentDialog`) _array_element)
      (:`then`
        (if (`|EnumEquality` (`.StatusAI_15_D793C07244CC91201393E4B9A9E73D5D` (break `/Game/Data/S_Dialog` _returnvalue)) "NewEnumerator5")
          (set `self.NumDialog` _array_index)
          (set `local.LHaveReactionReplica?` true)
          (break)))))
  (return (`local.LHaveReactionReplica?`)))

(fn `UserConstructionScript`)