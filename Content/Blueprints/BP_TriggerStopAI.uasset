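; Trigger volume that halts a BP_AI when it walks into the box and prepares it for its start dialog.
; On overlap it stops the AI's movement, changes its status, resets the start dialog and assigns the DT_StartDialog table.
; If a BP_CapsuleCharacter is already inside the AI's own box, the AI begins the dialog immediately.
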(event `self.Box.OnComponentBeginOverlap`
  (params (OverlappedComponent :type "PrimitiveComponent Object Reference") (OtherActor :type "Actor Object Reference") (OtherComp :type "PrimitiveComponent Object Reference") (OtherBodyIndex :type Integer) (bFromSweep :type Boolean) (SweepResult :type "HitResult Structure (by ref)"))
  (bind _asbp_ai (cast `/Game/Blueprints/BP_AI` OtherActor))
  (`/Game/Blueprints/BP_AI.StopMoving` _asbp_ai)
  (set `/Game/Blueprints/BP_AI.CurrentStatusAI` "NewEnumerator1" _asbp_ai)
  (`/Game/Blueprints/BP_AI.ResetStartDialog` _asbp_ai)
  (set `/Game/Blueprints/BP_AI.CurrentDialog` "/Game/Data/DT_StartDialog.DT_StartDialog" _asbp_ai)
  (if (> (`KismetArrayLibrary.Array_Length` (`PrimitiveComponent.GetOverlappingActors` (`/Game/Blueprints/BP_AI.Box` _asbp_ai) "/Game/Blueprints/BP_CapsuleCharacter.BP_CapsuleCharacter_C")) 0)
    (`/Game/Blueprints/BP_AI.StartBeginDialog` _asbp_ai)))

(fn `UserConstructionScript`)